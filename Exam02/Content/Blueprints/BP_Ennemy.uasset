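; BP_Ennemy is an enemy that takes damage and dies, animated with Skeleton King animations.
; It loops an idle animation from BeginPlay, playing animations directly on its skeletal mesh.
; The DamageTaken event plays a one-shot hit reaction, without returning to idle, and subtracts the damage from LifePoint.
; At zero or below, it plays the death animation and destroys the actor after a short delay.
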(event EventDamageTaken
  (params (DamageDo :type Float%20%28double-precision%29))
  (Components|Animation|PlayAnimation (Variables|Default|GetSkeletalMesh) "/Game/SkeletonCrew/Skeleton_King/Animations/Skeleton_King_Hit_Back.Skeleton_King_Hit_Back" false)
  (Variables|Default|SetLifePoint (- (Variables|Default|GetLifePoint) DamageDo))
  (if (<= (Variables|Default|GetLifePoint) 0.0)
    (Components|Animation|PlayAnimation (Variables|Default|GetSkeletalMesh) "/Game/SkeletonCrew/Skeleton_King/Animations/Skeleton_King_Death.Skeleton_King_Death" false)
    (Utilities|FlowControl|Delay 4.0)
    (Actor|DestroyActor)))

(event EventBeginPlay
  (Components|Animation|PlayAnimation (Variables|Default|GetSkeletalMesh) "/Game/SkeletonCrew/Skeleton_King/Animations/Skeleton_King_Idle_Loop.Skeleton_King_Idle_Loop" true))

(fn ConstructionScript)